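; AI controller Blueprint that starts behavior tree-driven AI for its controlled pawn.
; On BeginPlay it initializes BP_AIBlackboard and, if that succeeds, records the pawn's starting position as HomeLocation and sets a fixed AttackRange, provided the pawn is valid.
; It then runs the BP_AIBT behavior tree whether or not the pawn check passed; Tick and construction logic are empty.
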(event `self.ReceiveBeginPlay`
  (bind _returnvalue (`self.K2_GetPawn`))
  (bind (_blackboardcomponent _returnvalue_2) (`self.UseBlackboard` "/Game/Bluprint/AI/BP_AIBlackboard.BP_AIBlackboard"))
  (if _returnvalue_2
    (`|ExecutionSequence`
      (:`then_0`
        (`/Engine/EditorBlueprintResources/StandardMacros.IsValid` _returnvalue
          (:`Is Valid`
            (`BlackboardComponent.SetValueAsVector` _blackboardcomponent (`self.HomeLocation`) (`self.K2_GetActorLocation` _returnvalue))
            (`BlackboardComponent.SetValueAsFloat` _blackboardcomponent (`self.AttackRange`) 600.0))))
      (:`then_1`
        (`self.RunBehaviorTree` "/Game/Bluprint/AI/BP_AIBT.BP_AIBT")))))

(fn `UserConstructionScript`)