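; BP_AIPawn is an AI pawn Blueprint that keeps an enemy health widget up to date.
; On BeginPlay it sets its UI component to absolute rotation, binds to the OnUpdateHealthUI delegate and runs an initial refresh.
; UpdateHealthUI casts the widget component's user widget to UMG_EnemyHealth and passes the pawn to it, so the widget handles the display.
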(event `self.ReceiveBeginPlay`
  (set `SceneComponent.bAbsoluteRotation` true (`self.UI`))
  (`self.BindHealthUIDelegate`))

(fn `BindHealthUIDelegate`
  (add `self.OnUpdateHealthUI` (`|CreateDelegate` :!event `UpdateHealthUI`))
  (`self.UpdateHealthUI`))

(fn `UpdateHealthUI`
  (bind _asumg_enemy_health (cast `/Game/Bluprint/UMG/InGame/UMG_EnemyHealth` (`WidgetComponent.GetUserWidgetObject` (`self.Widget`))))
  (`/Game/Bluprint/UMG/InGame/UMG_EnemyHealth.UpdateHealthUI` _asumg_enemy_health self))

(fn `UserConstructionScript`)